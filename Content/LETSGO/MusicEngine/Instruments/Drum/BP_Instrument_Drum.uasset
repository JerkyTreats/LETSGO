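; Drum instrument Blueprint for the music engine that plays an 808 kick in time with a Quartz clock.
; On BeginPlay it gets the instrument's clock, subscribes to its beat quantization events and makes an initial QueueMusic call.
; QueueMusic, whose signature matches the quantization callback, spawns a new 2D kick MetaSound on each call and schedules it with PlayQuantized on that clock.
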(event Custom|QueueMusic
  (params (ClockName :type Name) (QuantizationType :type EQuartzCommandQuantization%20Enum :default "Bar") (NumBars :type Integer) (Beat :type Integer) (BeatFraction :type Float%20%28single-precision%29))
  (bind _returnvalue (Audio|SpawnSound2D "/Game/LETSGO/MusicEngine/Instruments/Drum/MS_Drum_Kick808.MS_Drum_Kick808" 1.0 1.0 0.0 0))
  (Audio|Components|Audio|PlayQuantized _returnvalue (Variables|Default|GetMainClock) (Utilities|Struct|MakeQuartzQuantizationBoundary "None" 1.0 "BarRelative") 0))

(event EventBeginPlay
  (bind _output_get (Variables|Default|SetMainClock (Class|Instrument|GetClock (Variables|Default|GetInstrument))))
  (Class|QuartzClockHandle|SubscribetoQuantizationEvent _output_get "Beat" (EventDispatchers|CreateEvent :!event Custom|QueueMusic))
  (CallFunction|QueueMusic "None" "None" 0 0 0.0))

(fn ConstructionScript)