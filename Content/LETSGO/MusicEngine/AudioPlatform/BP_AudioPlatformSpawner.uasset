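; Spawner actor that periodically drops short-lived audio platforms, each carrying a music note, intended to appear ahead of the player.
; On BeginPlay it fills an empty NoteContainer with notes from all generated D scales, then starts a looping timer.
; Each tick pops the next note and spawns a BP_AudioPlatform with it.
; A transform helper projects the pawn's location along the camera's horizontal forward direction at world height zero.
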(event Custom|Spawn%20Platform%20Task
  ;[1 1 1] Spawn Platforms Every X Seconds
  (CallFunction|SpawnPlatforminFrontOfPlayer))

(event EventBeginPlay
  ;[1 1 1] Determine if Notes is empty
  (if (> (Class|NoteContainer|GetNumberOfNotes (Variables|Default|GetNoteContainer)) 0)
    ;[1 1 1] Spawn Platforms Every X Seconds
    (Utilities|Time|SetTimerbyFunctionName 0 "Spawn Platform Task" 1.0 true :!label _label)
    (else
      ;[1 1 1] Generate Notes for All Scales
      (bind _returnvalue (Game|ConstructObjectfromClass "/Script/LETSGO.NoteContainer"))
      (Variables|Default|SetNoteContainer _returnvalue)
      (bind _returnvalue_2 (Class|LetsGoMusicEngine|GenerateAllScales (Utilities|Struct|MakeLetsGoMusicNotes "D")))
      (for _array_element _returnvalue_2
        ;[1 1 1] Add Notes to Note Container
        (Class|NoteContainer|AddNotes (Variables|Default|GetNoteContainer) (.Notes (Utilities|Struct|BreakLetsGoGeneratedScale _array_element)))
        (goto _label)))))

(fn ConstructionScript)

(fn SpawnPlatforminFrontOfPlayer
  (bind (_poppednote _returnvalue) (Class|NoteContainer|PopNextNote (Variables|Default|GetNoteContainer)))
  (if _returnvalue
    (Game|SpawnActorfromClass "/Game/LETSGO/MusicEngine/AudioPlatform/BP_AudioPlatform.BP_AudioPlatform_C" (Class|AudioPlatformSpawner|GetCameraVectorForward) "Undefined" "MultiplyWithRoot" 0 _poppednote 0.45 0)))

(fn GetVectorForwardTransform
  (bind _returnvalue (Game|GetPlayerController 0))
  (bind _returnvalue_2 (Game|GetPlayerCameraManager 0))
  (bind _returnvalue_3 (Pawn|GetControlledPawn _returnvalue))
  (bind _returnvalue_4 (Transformation|GetActorForwardVector _returnvalue_2))
  (bind _returnvalue_5 (Transformation|GetActorLocation _returnvalue_3))
  (bind _returnvalue_6 (* _returnvalue_4 "500.000000,500.000000,0.000000"))
  (bind _returnvalue_7 (+ _returnvalue_5 _returnvalue_6))
  (return (Math|Transform|MakeTransform (Math|Vector|MakeVector (.x _returnvalue_7) (.y _returnvalue_7) 0.0))))