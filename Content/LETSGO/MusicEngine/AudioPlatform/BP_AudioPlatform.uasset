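; BP_AudioPlatform is a music-engine platform actor that sounds its assigned note when the player character steps on it.
; On BeginPlay it adds a particle controller fed with its note, cube shape and AudioPlatform.
; Overlap fires the AudioPlatform trigger delegate, flags the platform as stepped on and activates the matching one of twelve chromatic note cues.
; After a fixed delay matching the note length, the actor destroys itself.
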(event Collision|EventActorBeginOverlap
  (params (OtherActor :type Actor%20Object%20Reference))
  (Utilities|Casting|CastToBP_ThirdPersonCharacter OtherActor)
  (Default|CallOnAudioPlatformTriggerDelegate (Variables|Default|GetAudioPlatform) (Variables|Default|GetMusicNote))
  (Variables|Default|SetHasBeenSteppedOn true)
  (switch Utilities|FlowControl|Switch|SwitchonELetsGoMusicNotes (Utilities|Struct|BreakLetsGoMusicNotes (Variables|Default|GetMusicNote))
    (:C
      (Components|Activation|Activate (Variables|Default|GetC3_Music_Note_Cue) false))
    (:CSharp
      (Components|Activation|Activate (Variables|Default|GetCSharp3_Music_Note_Cue) false))
    (:D
      (Components|Activation|Activate (Variables|Default|GetD_Music_Note_wav_Cue1) false))
    (:EFlat
      (Components|Activation|Activate (Variables|Default|GetEFlat2_Music_Note_Cue) false))
    (:E
      (Components|Activation|Activate (Variables|Default|GetE_Music_Note_Cue) false))
    (:F
      (Components|Activation|Activate (Variables|Default|GetF2_Music_Note_Cue) false))
    (:FSharp
      (Components|Activation|Activate (Variables|Default|GetFSharp2_Music_Note_Cue) false))
    (:G
      (Components|Activation|Activate (Variables|Default|GetG2_Music_Note_Cue) false))
    (:AFlat
      (Components|Activation|Activate (Variables|Default|GetAFlat2_Music_Note_Cue) false))
    (:A
      (Components|Activation|Activate (Variables|Default|GetA2_Music_Note_Cue) false))
    (:BFlat
      (Components|Activation|Activate (Variables|Default|GetBflat2_Music_Note_Cue) false))
    (:B
      (Components|Activation|Activate (Variables|Default|GetB2_Music_Note_Cue) false)))
  (Utilities|FlowControl|Delay 4.14) ; duration value == note length
  (Utilities|FlowControl|Sequence
    (:then_0
      (Actor|DestroyActor))))

(event EventBeginPlay
  (AddComponent|AddAudioPlatformParticleController (Variables|Default|GetMusicNote) (Variables|Default|GetShape_Cube) (Variables|Default|GetAudioPlatform)))

(fn ConstructionScript)