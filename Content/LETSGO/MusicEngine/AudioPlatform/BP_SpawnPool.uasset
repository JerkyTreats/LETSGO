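; BP_SpawnPool is a note queue for the LETSGO music engine's audio platform.
; Add Notes appends notes to the NotePool array, and Pop Next Note removes and returns the first one in FIFO order, with no empty check.
; BeginPlay is empty, and an unconnected chain that would fill the pool from every scale generated for a Tonic never runs.
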(event EventBeginPlay)

(fn PopNextNote
  (bind _note_pool (Variables|Default|GetNote%20Pool))
  (bind _output_get (Variables|Default|SetNext%20Note (Utilities|Array|Get(acopy) _note_pool)))
  (Utilities|Array|RemoveIndex _note_pool)
  (return _output_get))

(fn AddNotes
  (params (Notes :type Array%20of%20Lets%20Go%20Music%20Notes%20Structures))
  (Utilities|Array|AppendArray (Variables|Default|GetNote%20Pool) Notes))